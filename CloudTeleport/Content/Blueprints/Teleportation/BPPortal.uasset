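; BPPortal is a teleport portal actor that moves any Pawn entering its Teleportation component to another spot.
; On begin overlap it casts the other actor to Pawn and calls Teleport to a hardcoded location and zero rotation, printing a failure message for non-Pawns.
; A PortalDestination reference and several debug print and SetActorLocation chains sit unconnected, so they never affect the destination.
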(event `self.ReceiveBeginPlay`)

(event `self.Teleportation.OnComponentBeginOverlap`
  (params (OverlappedComponent :type "PrimitiveComponent Object Reference") (OtherActor :type "Actor Object Reference") (OtherComp :type "PrimitiveComponent Object Reference") (OtherBodyIndex :type Integer) (bFromSweep :type Boolean) (SweepResult :type "HitResult Structure (by ref)"))
  (bind _aspawn (cast `Pawn` OtherActor)
    (:`then`
      (`self.K2_TeleportTo` :`self` _aspawn :`DestLocation` (500.0 300.0 0.0)))
    (:`CastFailed`
      (`KismetSystemLibrary.PrintString` "cast failed" true true (struct :`R` 1.0 :`G` 0.072389 :`B` 0.062442 :`A` 1.0) 5.0))))

(fn `UserConstructionScript`)